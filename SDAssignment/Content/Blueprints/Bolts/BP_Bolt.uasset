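; BP_Bolt is a crossbow bolt projectile that damages what it hits and sticks to it.
; On a hit it sends damage and debuff type through BPI_Damageable, or makes noise and plays an impact sound for non-damageable targets.
; It then disables collision, attaches to the hit actor, and destroys itself when that actor is destroyed or after a short timer, with a lifespan as fallback.
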(event OnComponentHit(SM_Bolt_Base)
  (params (HitComponent :type Primitive%20Component%20Object%20Reference) (OtherActor :type Actor%20Object%20Reference) (OtherComp :type Primitive%20Component%20Object%20Reference) (NormalImpulse :type Vector :default "0, 0, 0") (Hit :type Hit%20Result%20Structure%20%28by%20ref%29))
  (bind _returnvalue (Transformation|GetActorLocation))
  (if (Utilities|DoesObjectImplementInterface OtherActor "/Game/Blueprints/Interfaces/BPI_Damageable.BPI_Damageable_C")
    (Class|BPIDamageable|DealDamage(Message) OtherActor (Variables|Default|GetDirectDamage) (Variables|Default|GetDebuffType))
    (else
      (Class|Actor|MakeNoise 1.0 0 _returnvalue 0.0 "None")
      (Audio|PlaySoundatLocation "/Game/Sound/Crossbow_Fire.Crossbow_Fire" _returnvalue "0, 0, 0" 0.5 1.0 0.1 0 0 0 0)))
  (Collision|SetCollisionEnabled (Variables|Default|GetSM_Bolt_Base) "NoCollision")
  (Transformation|AttachActorToActor OtherActor "None" "KeepWorld" "KeepWorld" "KeepWorld" false)
  (Utilities|IsValid OtherActor
    (:Is%20Valid
      (Game|AssignOnDestroyed OtherActor (delegate Custom|OnDestroyed_Event))
      (Utilities|Time|SetTimerbyEvent (delegate Custom|Cleanup) 4.0))
    (:Is%20Not%20Valid
      ;[0.15 0.15 0.15 0.5] Destroy bolt if the enemy dies, is invalid or after 4 seconds
      (Actor|DestroyActor))))

(event Custom|Cleanup
  ;[0.15 0.15 0.15 0.5] Destroy bolt if the enemy dies, is invalid or after 4 seconds
  (Actor|DestroyActor))

(event Custom|OnDestroyed_Event
  (params (DestroyedActor :type Actor%20Object%20Reference))
  ;[0.15 0.15 0.15 0.5] Destroy bolt if the enemy dies, is invalid or after 4 seconds
  (Actor|DestroyActor))

(event EventBeginPlay
  (Actor|SetLifeSpan 15.0))

(fn ConstructionScript)