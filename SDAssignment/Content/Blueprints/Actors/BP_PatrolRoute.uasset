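; BP_PatrolRoute is an actor that supplies world-space patrol points from a PatrolRoute spline.
; IncrementPatrolRoute advances PatrolIndex and wraps it to zero on reaching the spline point count, forming a loop.
; GetSplinePointAtWorldPosition returns the current point's world location.
; Direction logic for reversing is unfinished: the step only ever increments, and the -1 assignment is disconnected.
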(event Custom|IncrementPatrolRoute
  (bind _result (Math|Integer|IncrementInt (Variables|Default|GetPatrolIndex))
    (:%20%20
      (bind _output_get (Variables|Default|SetPatrolIndex _result))
      (if (== _output_get (Spline|GetNumberOfSplinePoints (Variables|Default|GetPatrolRoute)))
        (Variables|Default|SetPatrolIndex 0)
        (elif (== (Variables|Default|GetPatrolIndex) 0)
          (Variables|Default|SetDirection 1))))))

(fn ConstructionScript)

(fn GetSplinePointatWorldPosition
  (return (Spline|GetLocationatSplinePoint (Variables|Default|GetPatrolRoute) (Variables|Default|GetPatrolIndex) "World")))