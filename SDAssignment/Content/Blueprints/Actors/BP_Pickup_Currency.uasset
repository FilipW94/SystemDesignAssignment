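; Currency cache pickup actor that grants the player session currency.
; It overrides ApplyPickupEffect, acting only when the overlapping actor is player character 0 and returning whether the effect applied.
; On success it passes its CurrencyGained amount to the currency subsystem, tagged with an acquisition method, and increments the CurrencyCacheFound level stat.
; The event graph holds only disabled placeholder nodes.
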(event EventBeginPlay)

(event Collision|EventActorBeginOverlap
  (params (OtherActor :type Actor%20Object%20Reference))
  (|CallParentFunction OtherActor) ; This node is disabled and will not be called.\nDrag off pins to build functionality.
)

(event EventTick
  (params (DeltaSeconds :type Float%20%28single-precision%29)))

(fn ConstructionScript
  (|CallParentFunction))

(fn ApplyPickupEffect
  (params (OverlapActor :type Actor%20Object%20Reference))
  (if (== OverlapActor (Game|GetPlayerCharacter 0))
    (Class|CurrencySubsystem|IncreaseSessionCurrency (Subsystems|GetCurrencySubsystem) (Utilities|Struct|MakeAcquisition "Currency Cache Pickup" (Variables|Default|GetCurrency%20Gained)))
    (Class|LevelStatsSubsystem|IncrementLevelStat (Subsystems|GetLevelStatsSubsystem) "CurrencyCacheFound")
    (return true)
    (else
      (return false))))