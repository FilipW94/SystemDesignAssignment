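; BP_SaveTestActor is a debug actor that exercises the game instance's save system with a counter stored as PlayerCurrency.
; BeginPlay requests a load and enables input, with keys to create, save or load the save game.
; SaveData and LoadData events copy the counter, and the loaded callback bound by the load key reopens the current level.
; Overlapping the trigger mesh increments the counter, while Interact prints the initiator's name.
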(event OnComponentBeginOverlap(SM_VisibleTrigger)
  (params (OverlappedComponent :type Primitive%20Component%20Object%20Reference) (OtherActor :type Actor%20Object%20Reference) (OtherComp :type Primitive%20Component%20Object%20Reference) (OtherBodyIndex :type Integer) (bFromSweep :type Boolean) (SweepResult :type Hit%20Result%20Structure%20%28by%20ref%29))
  (bind _result (Math|Integer|IncrementInt (Variables|Default|GetSavedNumber))
    (:%20%20
      (Variables|Default|SetSavedNumber _result)
      (Development|PrintString (Utilities|String|ToString(Integer) (Variables|Default|GetSavedNumber))))))

(event Custom|GameLoaded_Event
  (params (SaveGameRef :type Prototype%20Save%20Game%20Object%20Reference))
  (bind _returnvalue (Game|GetCurrentLevelName true))
  (Game|OpenLevel(byName) (Utilities|String|StringToName _returnvalue)))

(event Custom|GameSaved_Event
  (params (SaveGameRef :type Prototype%20Save%20Game%20Object%20Reference))
  (Development|PrintString (Utilities|String|ToString(Integer) (Variables|Default|GetSavedNumber))))

(event EventBeginPlay
  (bind _asprototype_game_instance (Utilities|Casting|CastToPrototypeGameInstance (Game|GetGameInstance)))
  (bind _output_get (Variables|Default|SetGameInstanceRef _asprototype_game_instance))
  (Class|InterfacePersistence|RequestLoad _output_get self)
  (Input|EnableInput (Game|GetPlayerController 0)))

(event EventInteract
  (params (Initiator :type Actor%20Object%20Reference))
  (Development|PrintString (Utilities|GetDisplayName Initiator)))

(event EventSaveData
  (params (SaveGameRef :type Prototype%20Save%20Game%20Object%20Reference))
  (Variables|/Script/SDAssignment.PrototypeSaveGame|SetPlayerCurrency SaveGameRef (Variables|Default|GetSavedNumber)))

(event EventLoadData
  (params (SaveGameRef :type Prototype%20Save%20Game%20Object%20Reference))
  (Variables|Default|SetSavedNumber (Variables|/Script/SDAssignment.PrototypeSaveGame|GetPlayerCurrency SaveGameRef))
  (Development|PrintString (Utilities|String|ToString(Integer) (Variables|Default|GetSavedNumber))))

(event Input|KeyboardEvents|1
  (params (Key :type Key%20Structure :default "None"))
  (bind _gameinstanceref (Variables|Default|GetGameInstanceRef))
  (:Pressed
    (EventDispatchers|AssignGameSaved _gameinstanceref (delegate Custom|GameSaved_Event))
    (Class|InterfacePersistence|RequestSave(Message) _gameinstanceref false)
    (Development|PrintString (Utilities|String|ToString(Integer) (Variables|Default|GetSavedNumber)))))

(event Input|KeyboardEvents|2
  (params (Key :type Key%20Structure :default "None"))
  (bind _gameinstanceref (Variables|Default|GetGameInstanceRef))
  (:Pressed
    (EventDispatchers|AssignGameLoaded _gameinstanceref (delegate Custom|GameLoaded_Event))
    (Class|PrototypeGameInstance|LoadGame _gameinstanceref false)))

(event Input|KeyboardEvents|0
  (params (Key :type Key%20Structure :default "None"))
  (:Pressed
    (Class|PrototypeGameInstance|CreateSaveGame (Variables|Default|GetGameInstanceRef))))

(fn ConstructionScript)