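; Player crossbow weapon actor that fires bolts on left click while ammo remains and it is ready.
; Firing spawns the bolt class with its direct damage, makes noise, updates the HUD and level stats, then starts a timed reload.
; On BeginPlay it enables input and requests a game-instance load, whose callback adds unlocked bolt types to the available list.
; Setter functions adjust ammo, reload speed and damage.
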(event Custom|ReloadCrossBow
  (Class|BPIHUDCommunication|TriggerBoltReload(Message) (Variables|Default|GetHudRef) (Variables|Default|GetBoltReloadSpeed))
  (Utilities|Time|SetTimerbyEvent (delegate Custom|ReloadDone) (Variables|Default|GetBoltReloadSpeed)))

(event Custom|ReloadDone
  (Variables|Default|SetReadyToFire true))

(event Input|EnhancedActionEvents|EnhancedInputActionIA_LeftClick
  (params (ActionValue :type Boolean) (ElapsedSeconds :type Float%20%28double-precision%29) (TriggeredSeconds :type Float%20%28double-precision%29) (InputAction :type Input%20Action%20Object%20Reference :default "/Game/Input/IA_LeftClick.IA_LeftClick"))
  (if (> (Variables|Default|GetCurrentBolts) 0)
    (if (Variables|Default|GetReadyToFire)
      (CallFunction|FireBolt)
      (else
        (Development|PrintString "Crossbow not ready")))
    (else
      (Development|PrintString "Out of Bolts"))))

(event EventBeginPlay
  (bind _asplayer_controller (Utilities|Casting|CastToPlayerController (Game|GetInstigatorController (Components|GetOwner))))
  (Variables|Default|SetHudRef (HUD|GetHUD _asplayer_controller))
  (Input|EnableInput _asplayer_controller)
  (bind _asprototype_game_instance (Utilities|Casting|CastToPrototypeGameInstance (Game|GetGameInstance)))
  (bind _output_get (Variables|Default|SetGameInstanceRef _asprototype_game_instance))
  (Class|InterfacePersistence|RequestLoad _output_get self))

(event EventLoadData
  (params (SaveGameRef :type Prototype%20Save%20Game%20Object%20Reference))
  (bind _saved_unlockedbolts (Variables|/Script/SDAssignment.PrototypeSaveGame|GetSaved_UnlockedBolts SaveGameRef))
  (bind _keys (Utilities|Map|Keys _saved_unlockedbolts))
  (for _array_element _keys
    (if (.Value (Utilities|Map|Find _saved_unlockedbolts _array_element))
      (if (not (Utilities|Enum|Equal(Enum) _array_element "None"))
        (Utilities|Array|AddUnique (Variables|Default|GetAvailableBolts) _array_element)))))

(fn ConstructionScript)

(fn FireBolt
  (Variables|Default|SetReadyToFire false)
  (Game|SpawnActorfromClass (Variables|Default|GetBoltType) (Transformation|GetWorldTransform (Variables|Default|GetFiringPosition)) "AlwaysSpawn" "MultiplyWithRoot" 0 (Variables|Default|GetBoltDirectDamage) 0)
  (Class|Actor|MakeNoise 1.0 0 (Transformation|GetActorLocation) 0.0 "None")
  (bind _result (Math|Integer|DecrementInt (Variables|Default|GetCurrentBolts))
    (:%20%20
      (bind _output_get (Variables|Default|SetCurrentBolts _result))
      (Class|BPIHUDCommunication|UpdateBoltsRemaining(Message) (Variables|Default|GetHudRef) _output_get)
      (Class|LevelStatsSubsystem|IncrementLevelStat (Subsystems|GetLevelStatsSubsystem) "BoltsFired")
      (CallFunction|ReloadCrossBow))))

(fn SetStartingBolts
  (params (StartingBolts :type Integer))
  (Variables|Default|SetStartingBolts StartingBolts)
  (bind _output_get (Variables|Default|SetCurrentBolts (Variables|Default|GetStartingBolts)))
  (Class|BPIHUDCommunication|UpdateBoltsRemaining(Message) (Variables|Default|GetHudRef) _output_get))

(fn AddBolts
  (params (BoltsAdded :type Integer))
  (bind _output_get (Variables|Default|SetCurrentBolts (+ (Variables|Default|GetCurrentBolts) BoltsAdded)))
  (Class|BPIHUDCommunication|UpdateBoltsRemaining(Message) (Variables|Default|GetHudRef) _output_get))

(fn SetReloadSpeed
  (params (ReloadSpeed :type Float%20%28double-precision%29))
  (Variables|Default|SetBoltReloadSpeed ReloadSpeed))

(fn SetDirectDamage
  (params (DirectDamage :type Float%20%28double-precision%29))
  (Variables|Default|SetBoltDirectDamage DirectDamage))