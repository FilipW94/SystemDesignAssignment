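; Bolt pickup actor, a child pickup Blueprint that grants bolts to the actor that collects it.
; It overrides ApplyPickupEffect to send BoltsGained through the BPI_PickupEffect interface, increment the BoltCacheFound stat in the level stats subsystem, and return true.
; Only actors implementing that interface receive the effect, and its own event graph holds only disabled placeholder events.
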(event EventBeginPlay)

(event Collision|EventActorBeginOverlap
  (params (OtherActor :type Actor%20Object%20Reference))
  (|CallParentFunction OtherActor) ; This node is disabled and will not be called.\nDrag off pins to build functionality.
)

(event EventTick
  (params (DeltaSeconds :type Float%20%28single-precision%29)))

(fn ConstructionScript
  (|CallParentFunction))

(fn ApplyPickupEffect
  (params (OverlapActor :type Actor%20Object%20Reference))
  (if (Utilities|DoesObjectImplementInterface OverlapActor "/Game/Blueprints/Interfaces/BPI_PickupEffect.BPI_PickupEffect_C")
    (Class|BPIPickupEffect|BoltPickup(Message) OverlapActor (Variables|Default|GetBolts%20Gained))
    (Class|LevelStatsSubsystem|IncrementLevelStat (Subsystems|GetLevelStatsSubsystem) "BoltCacheFound")
    (return true)))