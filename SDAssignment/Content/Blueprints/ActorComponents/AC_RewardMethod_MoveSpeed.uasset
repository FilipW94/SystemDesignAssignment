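; Actor component for the move speed reward method, whose graph records the player's upgrade rank in the save game.
; SaveData scans saved upgrades for TableRowName and, on a match, removes index 0 rather than the matched index.
; It looks up the DT_Shop row named by TableRowName plus Rank, appends its UpgradeDetails and requests a save through the GameInstance.
; A missing row only prints an error.
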(event EventSaveData
  (params (SaveGameRef :type Prototype%20Save%20Game%20Object%20Reference))
  (bind _saved_playerupgrades (Variables|/Script/SDAssignment.PrototypeSaveGame|GetSaved_PlayerUpgrades SaveGameRef))
  (bind _array_element (Utilities|Array|ForEachLoopwithBreak _saved_playerupgrades :!label _label)
    (:LoopBody
      (if (== (.upgradename _array_element) (Variables|Default|GetTableRowName))
        (Utilities|Array|RemoveIndex _saved_playerupgrades)
        (goto _label Break)))
    (:Completed
      (bind _returnvalue (Utilities|GetDataTableRow "/Game/Blueprints/DT_Shop.DT_Shop" (Utilities|String|StringToName (Utilities|String|Append (Utilities|String|ToString(Name) (Variables|Default|GetTableRowName)) (Utilities|String|ToString(Integer) (Variables|Default|GetRank)))))
        (:then
          (Utilities|Array|Add (Variables|/Script/SDAssignment.PrototypeSaveGame|GetSaved_PlayerUpgrades SaveGameRef) (.upgradedetails _returnvalue))
          (bind _gameinstanceref (CallFunction|GetGameInstance))
          (Class|InterfacePersistence|RequestSave _gameinstanceref false))
        (:RowNotFound
          (Development|PrintString "Upgrade row not found"))))))