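; AC_Debuff is an actor component that represents a timed debuff on its owning actor.
; BeginPlay starts a timer for the debuff duration, and RefreshDebuff clears and restarts it.
; On expiry, RemoveDebuff sends the owner a removal message with the debuff type if it is valid, then destroys the component.
; The component also destroys itself with its owner and exposes the timer's remaining time.
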(event Custom|RefreshDebuff
  (Utilities|Time|ClearandInvalidateTimerbyHandle (Variables|Default|GetTimerHandle))
  (bind _returnvalue (Utilities|Time|SetTimerbyFunctionName 0 "RemoveDebuff" (Variables|Default|GetDebuffDuration)))
  (Variables|Default|SetTimerHandle _returnvalue))

(event Custom|OnDestroyed_Event
  (params (DestroyedActor :type Actor%20Object%20Reference))
  (Components|DestroyComponent))

(event EventBeginPlay
  (Game|AssignOnDestroyed (Components|GetOwner) (delegate Custom|OnDestroyed_Event))
  (bind _returnvalue (Utilities|Time|SetTimerbyFunctionName 0 "RemoveDebuff" (Variables|Default|GetDebuffDuration)))
  (Variables|Default|SetTimerHandle _returnvalue))

(fn GetRemaningDuration
  (return (Utilities|Time|GetTimerRemainingTimebyHandle (Variables|Default|GetTimerHandle))))

(fn RemoveDebuff
  (bind _returnvalue (Components|GetOwner))
  (Utilities|IsValid _returnvalue
    (:Is%20Valid
      (Class|BPIDamageable|RemoveDebuff(Message) _returnvalue (Variables|Default|GetDebuffType))
      (Components|DestroyComponent))
    (:Is%20Not%20Valid
      (Components|DestroyComponent))))