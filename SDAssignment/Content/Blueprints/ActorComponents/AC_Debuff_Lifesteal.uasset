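; Actor component debuff that drains health from its owner and gives it to player character 0.
; BeginPlay calls the parent, sets the debuff duration, then starts a timer whose event deals periodic damage, heals the player by the same amount and re-arms itself.
; RemoveDebuff applies one last damage and heal tick before calling the parent's removal.
; Damage and healing are both sent through message calls.
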(event Custom|DealPeriodicDamage
  (Class|BPIDamageable|DealDamage(Message) (Components|GetOwner) (Variables|Default|GetPeriodicDamage) "NewEnumerator0")
  (Class|BPIDamageable|HealDamage(Message) (Game|GetPlayerCharacter 0) (Variables|Default|GetPeriodicDamage))
  (Utilities|Time|SetTimerbyEvent (delegate Custom|DealPeriodicDamage) (Variables|Default|GetDamageTickIntervals)))

(event EventBeginPlay
  (|CallParentFunction)
  (Variables|Default|SetDebuffDuration 15.0)
  (Utilities|Time|SetTimerbyEvent (delegate Custom|DealPeriodicDamage) (Variables|Default|GetDamageTickIntervals)))

(fn RemoveDebuff
  (Class|BPIDamageable|DealDamage(Message) (Components|GetOwner) (Variables|Default|GetPeriodicDamage) "NewEnumerator0")
  (Class|BPIDamageable|HealDamage(Message) (Game|GetPlayerCharacter 0) (Variables|Default|GetPeriodicDamage))
  (|CallParentFunction))