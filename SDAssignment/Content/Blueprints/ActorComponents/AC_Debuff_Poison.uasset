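; Poison debuff actor component that deals periodic damage to its owner, extending a parent debuff component.
; BeginPlay runs the parent logic, sets the debuff duration and starts a timer that re-arms itself after each tick.
; Each tick sends the owner a damage message with a bolt type and prints a debug string.
; Removing the debuff deals one final hit of periodic damage before the parent's removal logic runs.
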(event Custom|DealPeriodicDamage
  (bind _periodicdamage (Variables|Default|GetPeriodicDamage))
  (Class|BPIDamageable|DealDamage(Message) (Components|GetOwner) _periodicdamage "NewEnumerator0")
  (Development|PrintString (Utilities|String|Append (Utilities|String|ToString(Float) _periodicdamage) " Poison damage dealt"))
  (Utilities|Time|SetTimerbyEvent (delegate Custom|DealPeriodicDamage) (Variables|Default|GetDamageTickIntervals)))

(event EventBeginPlay
  (|CallParentFunction)
  (Variables|Default|SetDebuffDuration 1e+01)
  (Utilities|Time|SetTimerbyEvent (delegate Custom|DealPeriodicDamage) (Variables|Default|GetDamageTickIntervals)))

(fn RemoveDebuff
  (Class|BPIDamageable|DealDamage(Message) (Components|GetOwner) (Variables|Default|GetPeriodicDamage) "NewEnumerator0")
  (|CallParentFunction))