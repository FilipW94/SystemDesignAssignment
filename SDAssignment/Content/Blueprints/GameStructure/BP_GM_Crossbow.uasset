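; Game mode for the Crossbow game that manages session currency, saving, player death and difficulty modifier getters.
; It clears session currency and loads the save on play, then banks session earnings into the total before restarting or returning to the menu.
; Death pauses play and shows the game-over screen.
; Resurrection resumes play and charges a currency-scaled cost, drawing on session funds before the saved total.
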(event Custom|NotifyPlayerDied_Event
  ;[0.15 0.15 0.15 0.5] Player Death
  (CallFunction|SetGameStatus true true true)
  (Class|BPIHUDCommunication|ShowGameOverScreen(Message) (HUD|GetHUD (Game|GetPlayerController 0))))

(event Custom|GameLoaded_Event
  (params (SaveGameRef :type Prototype%20Save%20Game%20Object%20Reference))
  (Development|PrintString "Game loaded"))

(event Custom|ResurrectPlayer
  ;[0.15 0.15 0.15 0.5] Player Death
  (Class|BPIDamageable|Resurrect(Message) (Game|GetPlayerCharacter 0))
  (CallFunction|SetGameStatus false false false)
  (CallFunction|SubtractResurrectCost))

(event Custom|SaveAndGoToMenu
  (bind _returnvalue (Subsystems|GetCurrencySubsystem))
  ;[0.15 0.15 0.15 0.5] Death Menu Logic
  (Class|CurrencySubsystem|IncreaseTotalCurrency _returnvalue (Class|CurrencySubsystem|GetSessionCurrency _returnvalue))
  (Class|InterfacePersistence|RequestSave (Variables|Default|GetGameInstanceRef) false)
  (Game|OpenLevel(byObjectReference) "/Game/Levels/LVL_MainMenu.LVL_MainMenu"))

(event Custom|RestartLevel
  (bind _returnvalue (Subsystems|GetCurrencySubsystem))
  ;[0.15 0.15 0.15 0.5] Death Menu Logic
  (Class|CurrencySubsystem|IncreaseTotalCurrency _returnvalue (Class|CurrencySubsystem|GetSessionCurrency _returnvalue))
  (Class|InterfacePersistence|RequestSave (Variables|Default|GetGameInstanceRef) false)
  (bind _returnvalue_2 (Game|GetCurrentLevelName true))
  (Game|OpenLevel(byName) (Utilities|String|StringToName _returnvalue_2)))

(event EventBeginPlay
  (Class|CurrencySubsystem|ClearSessionCurrency (Subsystems|GetCurrencySubsystem))
  (bind _asprototype_game_instance (Utilities|Casting|CastToPrototypeGameInstance (Game|GetGameInstance)))
  (Variables|Default|SetGameInstanceRef _asprototype_game_instance)
  (Class|PrototypeGameInstance|LoadGame (Variables|Default|GetGameInstanceRef) false)
  (EventDispatchers|AssignGameLoaded (Variables|Default|GetGameInstanceRef) (delegate Custom|GameLoaded_Event)))

(event EventSaveData
  (params (SaveGameRef :type Prototype%20Save%20Game%20Object%20Reference))
  ;[0.15 0.15 0.15 0.5] Save Currency
  (Variables|/Script/SDAssignment.PrototypeSaveGame|SetSaved_TotalResources SaveGameRef (Variables|/Script/SDAssignment.CurrencySubsystem|GetTotalCurrency (Subsystems|GetCurrencySubsystem))))

(fn ConstructionScript)

(fn CalculateResurrectCost
  (bind _returnvalue (Subsystems|GetCurrencySubsystem))
  (bind _output_get (Variables|Default|SetResurrectCost (+ (* (Variables|Default|GetBaseResurrectCost) (Variables|Default|GetEnemyCurrencyModifier)) (* (Class|CurrencySubsystem|GetSessionCurrency _returnvalue) 0.01) (* (Class|CurrencySubsystem|GetTotalCurrency _returnvalue) 0.01))))
  (return _output_get))

(fn SubtractResurrectCost
  (bind _returnvalue (Subsystems|GetCurrencySubsystem))
  (bind _returnvalue_2 (Class|CurrencySubsystem|GetSessionCurrency _returnvalue))
  (if (>= (Class|CurrencySubsystem|GetSessionCurrency (Subsystems|GetCurrencySubsystem)) (CallFunction|CalculateResurrectCost))
    (Class|CurrencySubsystem|DecreaseSessionCurrency (Subsystems|GetCurrencySubsystem) "Player Death" (Variables|Default|GetResurrectCost))
    (else
      (LocalVariables|SetRemaningCost (- (Variables|Default|GetResurrectCost) _returnvalue_2))
      (Class|CurrencySubsystem|DecreaseSessionCurrency _returnvalue "Player Death" _returnvalue_2)
      (Class|CurrencySubsystem|DecreaseTotalCurrency _returnvalue (LocalVariables|GetRemaningCost))
      (Class|InterfacePersistence|RequestSave (Variables|Default|GetGameInstanceRef) true))))

(fn SetGameStatus
  (params (PauseGame :type Boolean) (ShowMouse :type Boolean) (UIInputMode :type Boolean))
  (bind _returnvalue (Game|GetPlayerController 0))
  (Game|SetGamePaused PauseGame)
  (Variables|/Script/Engine.PlayerController|SetbShowMouseCursor (Game|GetPlayerController 0) ShowMouse)
  (if UIInputMode
    (Input|SetInputModeGameandUI _returnvalue 0 "DoNotLock" true false)
    (else
      (Input|SetInputModeGameOnly _returnvalue false)))
  (return))

(fn GetCurrencyModifier
  (return (Variables|Default|GetEnemyCurrencyModifier)))

(fn GetEnemyHealthModifier
  (return (Variables|Default|GetEnemyHealthModifer)))