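; HUD_Player is the player HUD, showing health, currency, crosshair reload animation and bolt count, plus the game over screen.
; Update events forward values to child widgets of WB_CombinedPlayerUI, with the currency total read from the currency subsystem.
; The combined UI is cached from PlayerHudWidgets' widget, with a timer retry if the cast fails.
; The game over widget is created on demand and replaces the player UI.
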(event EventBeginPlay
  (UserInterface|Viewport|AddtoViewport (CallFunction|GetPlayerUIWidget) 0)
  (CallFunction|UpdateTotalCurrency))

(event EventShowGameOverScreen
  (bind _gameoverwidgetref (CallFunction|GetGameOverWidget))
  (Widget|RemovefromParent (Variables|Default|GetPlayerUIRef))
  (UserInterface|Viewport|AddtoViewport _gameoverwidgetref 0)
  (Default|SetGameOverScreen _gameoverwidgetref))

(event EventUpdateTotalCurrency
  (Default|SetTotalCurrencyText (Variables|/Game/Widgets/WB_CombinedPlayerUI.WB_CombinedPlayerUI_C|GetWB_TotalCurrency (CallFunction|GetPlayerUIWidget)) (Class|CurrencySubsystem|GetTotalCurrency (Subsystems|GetCurrencySubsystem))))

(event EventUpdatePlayerHealth
  (params (CurrentHealth :type Float%20%28double-precision%29) (MaxHealth :type Float%20%28double-precision%29))
  (Default|SetPlayerHealthBar (Variables|/Game/Widgets/WB_CombinedPlayerUI.WB_CombinedPlayerUI_C|GetWB_PlayerHealthBar (Variables|Default|GetPlayerUIRef)) CurrentHealth MaxHealth))

(event EventTriggerBoltReload
  (params (ReloadTime :type Float%20%28double-precision%29))
  (Default|PlayReloadAnimation (Variables|/Game/Widgets/WB_CombinedPlayerUI.WB_CombinedPlayerUI_C|GetWB_Crosshair (Variables|Default|GetPlayerUIRef)) ReloadTime))

(event EventUpdateBoltsRemaining
  (params (BoltsRemaining :type Integer))
  (Default|SetBoltText (Variables|/Game/Widgets/WB_CombinedPlayerUI.WB_CombinedPlayerUI_C|GetWB_Bolts (Variables|Default|GetPlayerUIRef)) BoltsRemaining))

(fn ConstructionScript)

(fn GetPlayerUIWidget
  (Utilities|IsValid (Variables|Default|GetPlayerUIRef)
    (:Is%20Valid
      (return (Variables|Default|GetPlayerUIRef)))
    (:Is%20Not%20Valid
      (bind _aswb_combined_player_ui (Utilities|Casting|CastToWB_CombinedPlayerUI (UserInterface|GetWidget (Variables|Default|GetPlayerHudWidgets)))
        (:then
          (Variables|Default|SetPlayerUIRef _aswb_combined_player_ui)
          (return (Variables|Default|GetPlayerUIRef)))
        (:CastFailed
          (Utilities|Time|SetTimerbyFunctionName 0 "GetPlayerUIWidget" 0.1))))))

(fn GetGameOverWidget
  (Utilities|IsValid (Variables|Default|GetGameOverWidgetRef)
    (:Is%20Valid
      _)
    (:Is%20Not%20Valid
      (bind _returnvalue (UserInterface|CreateWidget "/Game/Widgets/WB_GameOver.WB_GameOver_C"))
      (Variables|Default|SetGameOverWidgetRef _returnvalue)))
  (return (Variables|Default|GetGameOverWidgetRef)))