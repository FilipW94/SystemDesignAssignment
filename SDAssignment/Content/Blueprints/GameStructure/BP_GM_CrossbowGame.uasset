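; BP_GM_CrossbowGame is the crossbow game's mode Blueprint, handling saving, player death and enemy modifiers.
; BeginPlay loads the save through PrototypeGameInstance and starts a timer that Autosave re-arms after requesting each save.
; SaveAndGoToMenu opens the main menu once the save callback fires, while player death pauses the game and shows the HUD's game-over screen.
; Getters expose enemy currency and health modifiers.
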(event Custom|NotifyPlayerDied_Event
  (Game|SetGamePaused true)
  (Class|BPIHUDCommunication|ShowGameOverScreen(Message) (HUD|GetHUD (Game|GetPlayerController 0))))

(event Custom|GameLoaded_Event
  (params (SaveGameRef :type Prototype%20Save%20Game%20Object%20Reference))
  (Development|PrintString "Game loaded"))

(event Custom|SaveAndGoToMenu
  (bind _gameinstanceref (Variables|Default|GetGameInstanceRef))
  (Class|InterfacePersistence|RequestSave _gameinstanceref false)
  (EventDispatchers|AssignGameSaved _gameinstanceref (delegate Custom|GameSaved_Event)))

(event Custom|Autosave
  (bind _gameinstanceref (Variables|Default|GetGameInstanceRef))
  ;[0.15 0.15 0.15 0.5] Autosave
  (EventDispatchers|AssignGameSaved _gameinstanceref (delegate Custom|GameSaved_Event_0))
  (Class|InterfacePersistence|RequestSave _gameinstanceref false)
  (Utilities|Time|SetTimerbyEvent (EventDispatchers|CreateEvent :!event Custom|Autosave) (Variables|Default|GetAutoSaveTimer)))

(event Custom|GameSaved_Event
  (params (SaveGameRef :type Prototype%20Save%20Game%20Object%20Reference))
  (Development|PrintString "Game saved.")
  (Game|OpenLevel(byObjectReference) "/Game/Levels/LVL_MainMenu.LVL_MainMenu"))

(event Custom|GameSaved_Event_0
  (params (SaveGameRef :type Prototype%20Save%20Game%20Object%20Reference))
  ;[0.15 0.15 0.15 0.5] Autosave
  (Development|PrintString "Autosaved"))

(event EventBeginPlay
  (bind _asprototype_game_instance (Utilities|Casting|CastToPrototypeGameInstance (Game|GetGameInstance)))
  (Variables|Default|SetGameInstanceRef _asprototype_game_instance)
  (Class|PrototypeGameInstance|LoadGame (Variables|Default|GetGameInstanceRef) false)
  (EventDispatchers|AssignGameLoaded (Variables|Default|GetGameInstanceRef) (delegate Custom|GameLoaded_Event))
  ;[0.15 0.15 0.15 0.5] Autosave
  (Utilities|Time|SetTimerbyEvent (EventDispatchers|CreateEvent :!event Custom|Autosave) (Variables|Default|GetAutoSaveTimer)))

(fn ConstructionScript)

(fn GetCurrencyModifier
  (return (Variables|Default|GetEnemyCurrencyModifier)))

(fn GetEnemyHealthModifier
  (return (Variables|Default|GetEnemyHealthModifer)))