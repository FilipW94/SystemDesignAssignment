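; Main menu game mode that loads persistent progression and starts levels the player has unlocked.
; On BeginPlay it requests a load through PrototypeGameInstance, pulling unlocked maps, total currency and player upgrade stats from the save.
; Saving writes back only unlocked maps and currency.
; StartLevel checks the unlock map, requests a save, and opens the level by name once the saved callback fires.
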(event Custom|GameLoaded_Event
  (params (SaveGameRef :type Prototype%20Save%20Game%20Object%20Reference))
  (Development|PrintString "Game loaded"))

(event Custom|StartLevel
  (params (Level :type E_Levels%20Enum :default "None") (LevelName :type Name))
  (bind _gameinstanceref (Variables|Default|GetGameInstanceRef))
  (bind _isunlocked (CallFunction|CheckMapUnlock Level))
  (if _isunlocked
    (EventDispatchers|AssignGameSaved _gameinstanceref (delegate Custom|GameSaved_Event))
    (Class|InterfacePersistence|RequestSave _gameinstanceref false)))

(event Custom|GameSaved_Event
  (params (SaveGameRef :type Prototype%20Save%20Game%20Object%20Reference))
  (Game|OpenLevel(byName) (stale Custom|StartLevel LevelName)))

(event EventSaveData
  (params (SaveGameRef :type Prototype%20Save%20Game%20Object%20Reference))
  (Variables|/Script/SDAssignment.PrototypeSaveGame|SetSaved_UnlockedMaps SaveGameRef (Variables|Default|GetMapsUnlocked))
  (Variables|/Script/SDAssignment.PrototypeSaveGame|SetSaved_TotalResources SaveGameRef (Variables|/Script/SDAssignment.CurrencySubsystem|GetTotalCurrency (Subsystems|GetCurrencySubsystem))))

(event EventLoadData
  (params (SaveGameRef :type Prototype%20Save%20Game%20Object%20Reference))
  (Variables|Default|SetMapsUnlocked (Variables|/Script/SDAssignment.PrototypeSaveGame|GetSaved_UnlockedMaps SaveGameRef))
  (Variables|/Script/SDAssignment.CurrencySubsystem|SetTotalCurrency (Subsystems|GetCurrencySubsystem) (Variables|/Script/SDAssignment.PrototypeSaveGame|GetSaved_TotalResources SaveGameRef))
  (Variables|Default|SetStartingBolts (Variables|/Script/SDAssignment.PrototypeSaveGame|GetSaved_StartingBolts SaveGameRef))
  (Variables|Default|SetDirectDamage (Variables|/Script/SDAssignment.PrototypeSaveGame|GetSaved_DirectDamage SaveGameRef))
  (Variables|Default|SetMaxHealth (Variables|/Script/SDAssignment.PrototypeSaveGame|GetSaved_MaxHealth SaveGameRef))
  (Variables|Default|SetReloadSpeed (Variables|/Script/SDAssignment.PrototypeSaveGame|GetSaved_ReloadSpeed SaveGameRef))
  (Variables|Default|SetMoveSpeed (Variables|/Script/SDAssignment.PrototypeSaveGame|GetSaved_MoveSpeed SaveGameRef)))

(event EventBeginPlay
  (bind _asprototype_game_instance (Utilities|Casting|CastToPrototypeGameInstance (Game|GetGameInstance)))
  (bind _output_get (Variables|Default|SetGameInstanceRef _asprototype_game_instance))
  (EventDispatchers|AssignGameLoaded _output_get (delegate Custom|GameLoaded_Event))
  (Class|InterfacePersistence|RequestLoad(Message) _output_get self))

(fn ConstructionScript)

(fn CheckMapUnlock
  (params (IsLevelUnlocked :type E_Levels%20Enum :default "None"))
  (return (.Value (Utilities|Map|Find (Variables|Default|GetMapsUnlocked) IsLevelUnlocked))))

(fn GetPlayerController
  (Utilities|IsValid (Variables|Default|GetPlayerControllerRef)
    (:Is%20Valid
      _)
    (:Is%20Not%20Valid
      (bind _asbp_pc_main_menu (Utilities|Casting|CastToBP_PC_MainMenu (Game|GetPlayerController 0)))
      (Variables|Default|SetPlayerControllerRef _asbp_pc_main_menu)))
  (return (Variables|Default|GetPlayerControllerRef)))