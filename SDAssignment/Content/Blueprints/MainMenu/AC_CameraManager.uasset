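; AC_CameraManager is a main menu component that supplies camera transforms for each menu screen.
; On BeginPlay it caches the transforms of reference actors for the main menu, level select, options, character and shop panes.
; GetDesiredLocation maps a requested menu type to its cached transform, leaving any actual camera movement to the caller.
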(event EventBeginPlay
  (Variables|Default|SetMainMenuLocation (Transformation|GetActorTransform (Variables|Default|GetMainMenuActor)))
  (Variables|Default|SetLevelSelectLocation (Transformation|GetActorTransform (Variables|Default|GetLevelSelectActor)))
  (Variables|Default|SetOptionsPaneLocation (Transformation|GetActorTransform (Variables|Default|GetOptionsPaneActor)))
  (Variables|Default|SetCharacterPaneLocation (Transformation|GetActorTransform (Variables|Default|GetCharacterPaneActor)))
  (Variables|Default|SetShopPaneLocation (Transformation|GetActorTransform (Variables|Default|GetShopPaneActor))))

(fn GetDesiredLocation
  (params (DesiredMenuType :type E_MenuType%20Enum :default "NewEnumerator0"))
  (switch Utilities|FlowControl|Switch|SwitchonE_MenuType DesiredMenuType
    (:NewEnumerator0
      (return (Variables|Default|GetMainMenuLocation)))
    (:NewEnumerator3
      (return (Variables|Default|GetLevelSelectLocation)))
    (:NewEnumerator2
      (return (Variables|Default|GetOptionsPaneLocation)))
    (:NewEnumerator4
      (return (Variables|Default|GetCharacterPaneLocation)))
    (:NewEnumerator1
      (return (Variables|Default|GetShopPaneLocation)))))