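; Main menu camera actor that becomes the player's view target and moves between menu screens such as main, level select, options, character select and shop.
; On BeginPlay it snaps to the first location supplied by the ACCameraManager component.
; Number keys 1–5 call AttemptTransition, which ignores requests mid-move, fetches the target transform from the manager and lerps the camera there with a timeline.
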(event Custom|TransitionCamera
  (Variables|Default|SetTransitionInProgress true)
  (bind _alpha (Timeline|TL_CameraTransition PlayFromStart)
    (:Update
      (Transformation|SetWorldTransform (Variables|Default|GetCamera) (Math|Transform|Lerp(Transform) (Variables|Default|GetCurrentTransform) (Variables|Default|GetDesiredTransform) _alpha) false false))
    (:Finished
      (Variables|Default|SetTransitionInProgress false))))

(event EventBeginPlay
  (bind _returnvalue (Game|GetPlayerController 0))
  (Input|EnableInput _returnvalue)
  (Game|Player|SetViewTargetwithBlend _returnvalue self 0.0 "VTBlend_Linear" 0.0 false)
  (bind _transform (Default|GetDesiredLocation (Variables|Default|GetAC_CameraManager) "NewEnumerator0"))
  (Transformation|SetWorldTransform (Variables|Default|GetCamera) _transform false true))

(event Input|KeyboardEvents|1
  (params (Key :type Key%20Structure :default "None"))
  ;[0.15 0.15 0.15 0.5] Main
  (:Pressed
    (CallFunction|AttemptTransition "NewEnumerator0")))

(event Input|KeyboardEvents|2
  (params (Key :type Key%20Structure :default "None"))
  ;[0.15 0.15 0.15 0.5] LevelSelect
  (:Pressed
    (CallFunction|AttemptTransition "NewEnumerator3")))

(event Input|KeyboardEvents|3
  (params (Key :type Key%20Structure :default "None"))
  ;[0.15 0.15 0.15 0.5] Options
  (:Pressed
    (CallFunction|AttemptTransition "NewEnumerator2")))

(event Input|KeyboardEvents|4
  (params (Key :type Key%20Structure :default "None"))
  ;[0.15 0.15 0.15 0.5] CharacterSelect
  (:Pressed
    (CallFunction|AttemptTransition "NewEnumerator4")))

(event Input|KeyboardEvents|5
  (params (Key :type Key%20Structure :default "None"))
  ;[0.15 0.15 0.15 0.5] ShopMenu
  (:Pressed
    (CallFunction|AttemptTransition "NewEnumerator1")))

(fn ConstructionScript)

(fn AttemptTransition
  (params (DesiredMenuLocation :type E_MenuType%20Enum :default "NewEnumerator6"))
  (if (not (Variables|Default|GetTransitionInProgress))
    (Variables|Default|SetCurrentTransform (Transformation|GetWorldTransform (Variables|Default|GetCamera)))
    (bind _transform (Default|GetDesiredLocation (Variables|Default|GetAC_CameraManager) DesiredMenuLocation))
    (Variables|Default|SetDesiredTransform _transform)
    (CallFunction|TransitionCamera)))

(fn GetMenuType
  (return "MenuPlacement_BelowAnchor"))