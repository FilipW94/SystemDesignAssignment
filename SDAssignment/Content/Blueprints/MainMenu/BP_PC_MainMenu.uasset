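; Main menu player controller that flies a single spawned camera between Main Menu, Level Select, Options, Character and Shop views.
; GetMenuType stores a camera transform per menu type, and BeginPlay makes the new camera the view target, placed at the Character transform.
; MoveCamera picks a stored transform and lerps to it on a timeline, ignoring requests mid-transition.
; Keys 1 and 2 trigger moves to Level Select and Character.
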(event Custom|TransitionCamera
  (Variables|Default|SetCameraTransitioning true)
  (bind _cameralerpalpha (Timeline|TL_TransitionCamera PlayFromStart)
    (:Update
      (Transformation|SetActorTransform (Variables|Default|GetMainMenuCamera) (Math|Transform|Lerp(Transform) (Variables|Default|GetCurrentTransform) (Variables|Default|GetDesiredTransform) _cameralerpalpha)))
    (:Finished
      (Variables|Default|SetCameraTransitioning false))))

(event EventMoveCamera
  (params (MoveToLocation :type E_MenuLocations%20Enum :default "NewEnumerator6"))
  (if (not (Variables|Default|GetCameraTransitioning))
    (Variables|Default|SetCurrentTransform (Transformation|GetActorTransform (Variables|Default|GetMainMenuCamera)))
    (switch Utilities|FlowControl|Switch|SwitchonE_MenuLocations MoveToLocation
      (:NewEnumerator0
        (Variables|Default|SetDesiredTransform (Variables|Default|GetMainMenuTransform)))
      (:NewEnumerator3
        (Variables|Default|SetDesiredTransform (Variables|Default|GetLevelSelectTransform)))
      (:NewEnumerator2
        (Variables|Default|SetDesiredTransform (Variables|Default|GetOptionsTransform)))
      (:NewEnumerator4
        (Variables|Default|SetDesiredTransform (Variables|Default|GetCharacterTransform)))
      (:NewEnumerator1
        (Variables|Default|SetDesiredTransform (Variables|Default|GetShopTransform))))
    (CallFunction|TransitionCamera)))

(event EventGetMenuType
  (params (MenuType :type E_MenuLocations%20Enum :default "NewEnumerator6") (CameraTransform :type Transform))
  (switch Utilities|FlowControl|Switch|SwitchonE_MenuLocations MenuType
    (:NewEnumerator0
      (Variables|Default|SetMainMenuTransform CameraTransform))
    (:NewEnumerator3
      (Variables|Default|SetLevelSelectTransform CameraTransform))
    (:NewEnumerator2
      (Variables|Default|SetOptionsTransform CameraTransform))
    (:NewEnumerator4
      (Variables|Default|SetCharacterTransform CameraTransform))
    (:NewEnumerator1
      (Variables|Default|SetShopTransform CameraTransform))))

(event EventBeginPlay
  (bind _returnvalue (Game|SpawnActorfromClass "/Script/Engine.CameraActor" (Math|Transform|MakeTransform "0, 0, 0" "0, 0, 0" "1.000000,1.000000,1.000000") "AlwaysSpawn" "MultiplyWithRoot" 0 0))
  (bind _output_get (Variables|Default|SetMainMenuCamera _returnvalue))
  (Game|Player|SetViewTargetwithBlend _output_get 0.0 "VTBlend_Linear" 0.0 false)
  (Transformation|SetActorTransform (Variables|Default|GetMainMenuCamera) (Variables|Default|GetCharacterTransform) false true))

(event Input|KeyboardEvents|1
  (params (Key :type Key%20Structure :default "None"))
  (:Pressed
    (CallFunction|MoveCamera "NewEnumerator3")))

(event Input|KeyboardEvents|2
  (params (Key :type Key%20Structure :default "None"))
  (:Pressed
    (CallFunction|MoveCamera "NewEnumerator4")))

(fn ConstructionScript)